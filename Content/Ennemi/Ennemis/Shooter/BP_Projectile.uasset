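; Projectile for the Shooter enemy that damages the player's SideScrollerCharacter on contact.
; Tick moves it along its root's forward vector at a fixed speed without sweep, and a Delay in the same chain destroys it after a few seconds.
; Hitbox overlap applies Damage to the player and destroys the projectile, which passes through CH_Ennemis actors and is destroyed by any other overlap.
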(event OnComponentBeginOverlap(projectilhitbox)
  (params (OverlappedComponent :type Primitive%20Component%20Object%20Reference) (OtherActor :type Actor%20Object%20Reference) (OtherComp :type Primitive%20Component%20Object%20Reference) (OtherBodyIndex :type Integer) (bFromSweep :type Boolean) (SweepResult :type Hit%20Result%20Structure%20%28by%20ref%29))
  (bind _asside_scroller_character (Utilities|Casting|CastToSideScrollerCharacter OtherActor)
    (:then
      (Game|Damage|ApplyDamage _asside_scroller_character (Math|Conversions|ToFloat(Integer) (Variables|Default|GetDamage)) 0 0)
      (Actor|DestroyActor))
    (:CastFailed
      (Utilities|Casting|CastToCH_Ennemis OtherActor
        (:CastFailed
          (Actor|DestroyActor))))))

(event EventTick
  (params (DeltaSeconds :type Float%20%28single-precision%29))
  (Transformation|AddActorWorldOffset (* (Math|Vector|GetForwardVector (Variables|Default|GetDefaultSceneRoot)) (* DeltaSeconds 3e+02)))
  ;[1 0.8011 0.06383] Durée de vie du projectile
  (Utilities|FlowControl|Delay 7.5)
  (Actor|DestroyActor))

(fn ConstructionScript)